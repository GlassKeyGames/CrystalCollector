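; BP_Crystal is a collectible crystal pickup that spins every tick.
; On sphere overlap with BP_ThirdPersonCharacter, it increments that character's crystal count and calls WinGame once the count reaches the character's total.
; It then updates the character's HUD widget, plays a pickup sound at its location and destroys itself.
; The spin is a fixed per-frame local rotation, not scaled by delta time.
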(event `self.SphereCollision.OnComponentBeginOverlap`
  (params (OverlappedComponent :type "PrimitiveComponent Object Reference") (OtherActor :type "Actor Object Reference") (OtherComp :type "PrimitiveComponent Object Reference") (OtherBodyIndex :type Integer) (bFromSweep :type Boolean) (SweepResult :type "HitResult Structure (by ref)"))
  (bind _asbp_third_person_character (cast `/Game/Characters/ThirdPerson/Blueprints/BP_ThirdPersonCharacter` OtherActor))
  (bind _crystalscollected (`/Game/Characters/ThirdPerson/Blueprints/BP_ThirdPersonCharacter.CrystalsCollected` _asbp_third_person_character))
  (bind _output_get (set `/Game/Characters/ThirdPerson/Blueprints/BP_ThirdPersonCharacter.CrystalsCollected` (+ _crystalscollected 1) _asbp_third_person_character))
  (if (>= _crystalscollected (`/Game/Characters/ThirdPerson/Blueprints/BP_ThirdPersonCharacter.TotalCrystals` _asbp_third_person_character))
    (`/Game/Characters/ThirdPerson/Blueprints/BP_ThirdPersonCharacter.WinGame` _asbp_third_person_character))
  (`/Game/CrystalCollector/UI/WBP_HUD.UpdateCrystalCount` (`/Game/Characters/ThirdPerson/Blueprints/BP_ThirdPersonCharacter.HUDWidget` _asbp_third_person_character) _output_get)
  (`GameplayStatics.PlaySoundAtLocation` "/Game/CrystalCollector/Audio/SFX_CrystalPickup.SFX_CrystalPickup" (`self.K2_GetActorLocation`) (struct) 1.0 1.0 0.0 null null null null)
  (`self.K2_DestroyActor`))

(event `self.ReceiveTick`
  (params (DeltaSeconds :type "Float (single-precision)"))
  (`self.K2_AddActorLocalRotation` (struct :`Yaw` 3.0 :`Roll` 3.0)))

(fn `UserConstructionScript`)